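; BP_MoveRect is an actor that moves its Cube component around a square loop in the relative X-Z plane.
; While IsPlay is true, Tick switches on a MoveType state, offsets the cube by Speed times delta time and advances to the next side when a fixed bound is passed.
; EventPlay and EventStop set IsPlay to start and pause the motion.
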(event `self.ReceiveTick`
  (params (DeltaSeconds :type "Float (single-precision)"))
  (bind _returnvalue (* DeltaSeconds (`self.Speed`)))
  (bind (_relativelocation_x _relativelocation_y _relativelocation_z) (`KismetMathLibrary.BreakVector` (`SceneComponent.RelativeLocation` (`self.Cube`))))
  (bind _relativelocation_x_2 (`KismetMathLibrary.BreakVector` (`SceneComponent.RelativeLocation` (`self.Cube`))))
  (bind _relativelocation_x_3 (`KismetMathLibrary.BreakVector` (`SceneComponent.RelativeLocation` (`self.Cube`))))
  (bind (_relativelocation_x_4 _relativelocation_y_2 _relativelocation_z_2) (`KismetMathLibrary.BreakVector` (`SceneComponent.RelativeLocation` (`self.Cube`))))
  (bind _returnvalue_2 (* _returnvalue -1.0))
  (if (`self.IsPlay`)
    (switch `/Game/Project/EN_MoveType` (`self.MoveType`)
      (:`NewEnumerator0`
        (`SceneComponent.K2_AddRelativeLocation` (`self.Cube`) (`KismetMathLibrary.MakeVector` _returnvalue) false false)
        (if (>= _relativelocation_x_3 200.0)
          (set `self.MoveType` "NewEnumerator1")))
      (:`NewEnumerator1`
        (`SceneComponent.K2_AddRelativeLocation` (`self.Cube`) (`KismetMathLibrary.MakeVector` 0.0 0.0 _returnvalue) false false)
        (if (>= _relativelocation_z 200.0)
          (set `self.MoveType` "NewEnumerator2")))
      (:`NewEnumerator2`
        (`SceneComponent.K2_AddRelativeLocation` (`self.Cube`) (`KismetMathLibrary.MakeVector` _returnvalue_2) false false)
        (if (<= _relativelocation_x_2 0.0)
          (set `self.MoveType` "NewEnumerator3")))
      (:`NewEnumerator3`
        (`SceneComponent.K2_AddRelativeLocation` (`self.Cube`) (`KismetMathLibrary.MakeVector` 0.0 0.0 _returnvalue_2) false false)
        (if (<= _relativelocation_z_2 0.0)
          (set `self.MoveType` "NewEnumerator0"))))))

(event `/Game/Project/BPI_MoveActor.EventPlay`
  (set `self.IsPlay` true))

(event `/Game/Project/BPI_MoveActor.EventStop`
  (set `self.IsPlay` false))

(fn `UserConstructionScript`)