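; BP_MoveLeftRight is a Blueprint that slides its Cube component back and forth along the local X axis.
; While IsPlay is set, Tick moves the cube by Speed scaled by delta time, for frame-rate-independent motion.
; The IsRight flag reverses at fixed relative-X limits, checked after each move without clamping.
; EventPlay and EventStop toggle IsPlay to resume or pause the motion.
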(event `self.ReceiveTick`
  (params (DeltaSeconds :type "Float (single-precision)"))
  (bind _returnvalue (* DeltaSeconds (`self.Speed`)))
  (bind _relativelocation_x (`KismetMathLibrary.BreakVector` (`SceneComponent.RelativeLocation` (`self.Cube`))))
  (bind _relativelocation_x_2 (`KismetMathLibrary.BreakVector` (`SceneComponent.RelativeLocation` (`self.Cube`))))
  (if (`self.IsPlay`)
    (if (`self.IsRight`)
      (`SceneComponent.K2_AddRelativeLocation` (`self.Cube`) (`KismetMathLibrary.MakeVector` _returnvalue) false false)
      (if (>= _relativelocation_x_2 200.0)
        (set `self.IsRight` false))
      (else
        (`SceneComponent.K2_AddRelativeLocation` (`self.Cube`) (`KismetMathLibrary.MakeVector` (* _returnvalue -1.0)) false false)
        (if (<= _relativelocation_x 0.0)
          (set `self.IsRight` true))))))

(event `/Game/Project/BPI_MoveActor.EventPlay`
  (set `self.IsPlay` true))

(event `/Game/Project/BPI_MoveActor.EventStop`
  (set `self.IsPlay` false))

(fn `UserConstructionScript`)