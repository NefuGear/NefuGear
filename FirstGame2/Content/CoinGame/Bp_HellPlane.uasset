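; Fire hazard plane that damages the player while their third-person character overlaps it, with a fire emitter spawned at its location on BeginPlay.
; Overlap start runs a fast looping timer on the HellPlane function, which calls AddDamage on player 0's BP_PlayerState in small increments.
; Any actor ending overlap re-sets that timer with no time given, which clears it and stops the damage.
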(event `self.Plane.OnComponentBeginOverlap`
  (params (OverlappedComponent :type "PrimitiveComponent Object Reference") (OtherActor :type "Actor Object Reference") (OtherComp :type "PrimitiveComponent Object Reference") (OtherBodyIndex :type Integer) (bFromSweep :type Boolean) (SweepResult :type "HitResult Structure (by ref)"))
  (cast `/Game/ThirdPerson/Blueprints/BP_ThirdPersonCharacter` OtherActor)
  (`KismetSystemLibrary.K2_SetTimer` null "HellPlane" 0.01 true))

(event `self.Plane.OnComponentEndOverlap`
  (params (OverlappedComponent :type "PrimitiveComponent Object Reference") (OtherActor :type "Actor Object Reference") (OtherComp :type "PrimitiveComponent Object Reference") (OtherBodyIndex :type Integer))
  (`KismetSystemLibrary.K2_SetTimer` null "HellPlane"))

(event `self.ReceiveBeginPlay`
  (bind (_returnvalue_location _returnvalue_rotation) (`KismetMathLibrary.BreakTransform` (`self.GetTransform`)))
  (`GameplayStatics.SpawnEmitterAtLocation` "/Game/StarterContent/Particles/P_Fire.P_Fire" _returnvalue_location _returnvalue_rotation (2.0 2.0 2.0)))

(fn `HellPlane`
  (bind _asbp_player_state (cast `/Game/CoinGame/GameMode/BP_PlayerState` (`GameplayStatics.GetPlayerState` 0)))
  (`/Game/CoinGame/GameMode/BP_PlayerState.AddDamage` _asbp_player_state 0.01))

(fn `UserConstructionScript`)