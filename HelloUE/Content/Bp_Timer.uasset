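; Timer Blueprint that counts elapsed time and prints it on screen as a zero-padded minutes:seconds string.
; Tick accumulates delta seconds into a total and passes it to MinSec, which formats each part through a pad-to-two-digits helper.
; MinSec prints only when the string differs from the last one stored, so output updates once per second.
; Earlier formatting attempts, including four digit-case print functions, remain as disconnected practice nodes.
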(event `self.ReceiveTick`
  (params (DeltaSeconds :type "Float (single-precision)"))
  ;[1 1 1] 함수 활용 분초 계산
  (bind _output_get (set `self.TotalSec` (+ (`self.TotalSec`) DeltaSeconds)))
  (`self.Min Sec` _output_get _output_get))

(fn `0N:0N`
  (params (B :type String) (B2 :type String))
  (`KismetSystemLibrary.PrintString` (`KismetStringLibrary.Concat_StrStr` (`KismetStringLibrary.Concat_StrStr` "0" B) ":" (`KismetStringLibrary.Concat_StrStr` "0" B2))))

(fn `0N:NN`
  (params (B :type String) (C :type String))
  (`KismetSystemLibrary.PrintString` (`KismetStringLibrary.Concat_StrStr` (`KismetStringLibrary.Concat_StrStr` "0" B) ":" C)))

(fn `Float to Str 00`
  (params (Number :type "Float (double-precision)"))
  (returns (str00 :type String))
  (bind _returnvalue (`KismetMathLibrary.FFloor` Number))
  (if (< _returnvalue 10)
    (return (`KismetStringLibrary.Concat_StrStr` "0" (`KismetStringLibrary.Conv_IntToString` _returnvalue))) ; 결과는 '0N'
    (else
      (return (`KismetStringLibrary.Conv_IntToString` _returnvalue)) ; 결과는 'NN'
    )))

(fn `Min Sec`
  (params (A :type "Float (double-precision)") (A2 :type "Float (double-precision)"))
  (bind _str00 (`self.Float to Str 00` (/ A 60.0))) ; 초 단위
  (bind _str00_2 (`self.Float to Str 00` (mod A2 60.0))) ; 분 단위
  (bind _returnvalue (`KismetStringLibrary.Concat_StrStr` _str00 ":" _str00_2))
  (if (not (== (`self.beforString`) _returnvalue))
    (`KismetSystemLibrary.PrintString` _returnvalue true true (struct :`G` 0.66 :`B` 1.0 :`A` 1.0) 0.99)
    (set `self.beforString` _returnvalue)))

(fn `NN:0N`
  (params (B :type String) (A :type String))
  (`KismetSystemLibrary.PrintString` (`KismetStringLibrary.Concat_StrStr` A ":" (`KismetStringLibrary.Concat_StrStr` "0" B))))

(fn `NN:NN`
  (params (A :type String) (C :type String))
  (`KismetSystemLibrary.PrintString` (`KismetStringLibrary.Concat_StrStr` A ":" C)))

(fn `UserConstructionScript`)