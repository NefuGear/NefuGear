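; Bp_HelloLv is a practice Blueprint that slides a Sphere component back and forth along its relative X axis.
; Each Tick moves the sphere by Speed scaled by delta time, and the IsMoveRight flag flips when it reaches either fixed end of the range.
; The rest of the event graph is disconnected scratch nodes testing printing, loops, variables, delay and transforms, none of which run.
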(event `self.ReceiveBeginPlay`)

(event `self.ReceiveTick`
  (params (DeltaSeconds :type "Float (single-precision)"))
  (bind _sphere (`self.Sphere`))
  (bind _sphere_2 (`self.Sphere`))
  (bind _relativelocation_x (`KismetMathLibrary.BreakVector` (`SceneComponent.RelativeLocation` _sphere)))
  (bind _relativelocation_x_2 (`KismetMathLibrary.BreakVector` (`SceneComponent.RelativeLocation` _sphere_2)))
  (if (`self.IsMoveRight`)
    ;[0 0.08041 1] 오른쪽으로 이동
    (`SceneComponent.K2_AddRelativeLocation` _sphere (`KismetMathLibrary.MakeVector` (* DeltaSeconds (`self.speed`))) false false)
    (if (>= _relativelocation_x 200.0)
      (set `self.IsMoveRight` false))
    (else
      ;[1 0 0.07867] 왼쪽으로 이동
      (`SceneComponent.K2_AddRelativeLocation` _sphere_2 (`KismetMathLibrary.MakeVector` (* (* DeltaSeconds (`self.speed`)) -1.0)) false false)
      (if (<= _relativelocation_x_2 0.0)
        (set `self.IsMoveRight` true)))))

(fn `UserConstructionScript`)