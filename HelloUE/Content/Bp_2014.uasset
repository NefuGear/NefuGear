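; Blueprint with logic for looping a Sphere around a square in its relative XZ plane, currently inert because BeginPlay and Tick are empty.
; A disconnected switch on the Seter direction state calls four move functions, each offsetting the Sphere by speed times delta time.
; Each function advances Seter at its bound, cycling Right, Up, Left, Down.
; Other unwired fragments include an elapsed-time print and a rotation step.
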(event `self.ReceiveBeginPlay`)

(event `self.ReceiveTick`
  (params (DeltaSeconds :type "Float (single-precision)")))

(fn `Move Left`
  (params (A :type "Float (double-precision)") (B :type "Float (double-precision)") (InputPin :type "StaticMeshComponent Object Reference") (InputPin2 :type Boolean))
  (`SceneComponent.K2_AddRelativeLocation` InputPin (`KismetMathLibrary.MakeVector` (* (* A B) -1.0)) false false)
  (if InputPin2
    (set `self.Seter` "NewEnumerator7")))

(fn `Move Right`
  (params (A :type "Float (double-precision)") (B :type "Float (double-precision)") (self2 :type "SceneComponent Object Reference") (Condition :type Boolean))
  (`SceneComponent.K2_AddRelativeLocation` self2 (`KismetMathLibrary.MakeVector` (* A B)) false false)
  (if Condition
    (set `self.Seter` "NewEnumerator5")))

(fn `NewFunction`
  (params (A :type "Float (double-precision)") (B :type "Float (double-precision)") (self2 :type "SceneComponent Object Reference") (Condition :type Boolean))
  (`SceneComponent.K2_AddRelativeLocation` self2 (`KismetMathLibrary.MakeVector` 0.0 0.0 (* A B)) false false)
  (if Condition
    (set `self.Seter` "NewEnumerator6")))

(fn `NewFunction_0`
  (params (A :type "Float (double-precision)") (B :type "Float (double-precision)") (Condition :type Boolean) (InputPin :type "StaticMeshComponent Object Reference"))
  (`SceneComponent.K2_AddRelativeLocation` InputPin (`KismetMathLibrary.MakeVector` 0.0 0.0 (* (* A B) -1.0)) false false)
  (if Condition
    (set `self.Seter` "NewEnumerator4")))

(fn `UserConstructionScript`)