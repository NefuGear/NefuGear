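; Coin game state Blueprint that tracks elapsed play time and shows it as a minutes:seconds timer on the HUD.
; Each Tick, PrintTime adds delta seconds to TotalSec and splits it into minutes and seconds.
; FloatToStr00 floors each value and zero-pads it below ten before the joined text goes to Bp_HUD's SetTimeText through player controller 0.
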(event `self.ReceiveTick`
  (params (DeltaSeconds :type "Float (single-precision)"))
  (`self.PrintTime` DeltaSeconds))

(fn `Float to Str 00`
  (params (Number :type "Float (double-precision)"))
  (returns (str00 :type String))
  (locals (NewLocalVar :type String))
  (bind _returnvalue (`KismetMathLibrary.FFloor` Number))
  (if (< _returnvalue 10)
    (return (`KismetStringLibrary.Concat_StrStr` "0" (`KismetStringLibrary.Conv_IntToString` _returnvalue))) ; 결과는 '0N'
    (else
      (return (`KismetStringLibrary.Conv_IntToString` _returnvalue)) ; 결과는 'NN'
    )))

(fn `PrintTime`
  (params (NewParam :type "Float (double-precision)"))
  (bind _output_get (set `self.TotalSec` (+ NewParam (`self.TotalSec`))))
  (bind _str00 (`self.Float to Str 00` (/ _output_get 60.0))) ; 초 단위
  (bind _str00_2 (`self.Float to Str 00` (mod _output_get 60.0))) ; 분 단위
  (bind _asbp_hud (cast `/Game/CoinGame/GameMode/Bp_HUD` (`PlayerController.GetHUD` (`GameplayStatics.GetPlayerController` 0))))
  (`/Game/CoinGame/GameMode/Bp_HUD.SetTimeText` _asbp_hud (`KismetStringLibrary.Concat_StrStr` _str00 ":" _str00_2)))

(fn `UserConstructionScript`)