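; Player state Blueprint for the coin game that keeps counts of collected coins and red items.
; AddCoins increments Coin, then casts player 0's HUD to Bp_HUD and passes it the new total through SetCoinText.
; AddRedItem increments RedItem and performs the same cast but makes no HUD update.
; BeginPlay, Tick and the construction script are empty.
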(fn `Add Coins`
  (bind _output_get (set `self.coin` (+ (`self.coin`) 1)))
  (bind _asbp_hud (cast `/Game/CoinGame/GameMode/Bp_HUD` (`PlayerController.GetHUD` (`GameplayStatics.GetPlayerController` 0))))
  (`/Game/CoinGame/GameMode/Bp_HUD.SetCoinText` _asbp_hud _output_get))

(fn `Add Red Item`
  (set `self.RedItem` (+ (`self.RedItem`) 1))
  (cast `/Game/CoinGame/GameMode/Bp_HUD` (`PlayerController.GetHUD` (`GameplayStatics.GetPlayerController` 0))))

(fn `UserConstructionScript`)