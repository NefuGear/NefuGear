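; Collectible coin actor that adds a coin to the overlapping BP_ThirdPersonCharacter1 and respawns after a short delay.
; On pickup it hides the Cylinder, disables its collision, notifies the Portal, and sets a timer to run showcoin.
; BeginPlay adds a CoinCount widget to the viewport.
; CustomEvent_1, not called here, starts timer-driven spinning, finds Portal by the "BTS" tag and adds further CoinCount widgets.
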(event `self.ReceiveTick`
  (params (DeltaSeconds :type "Float (single-precision)"))
  ;[1 1 1] 코멘트
)

(event `self.ReceiveBeginPlay`
  ;[1 1 1] 코멘트
  ;;[1 1 1] 변형
  (bind _returnvalue (`|CreateWidget` "/Game/Project/coin/CoinCount.CoinCount_C"))
  (bind _output_get (set `self.text` _returnvalue))
  (`UserWidget.AddToViewport` _output_get 0)
  (`UserWidget.AddToViewport` _returnvalue 0)
  (for _ (range 10)
    _))

(event `self.Cylinder.OnComponentBeginOverlap`
  (params (OverlappedComponent :type "PrimitiveComponent Object Reference") (OtherActor :type "Actor Object Reference") (OtherComp :type "PrimitiveComponent Object Reference") (OtherBodyIndex :type Integer) (bFromSweep :type Boolean) (SweepResult :type "HitResult Structure (by ref)"))
  (bind _cylinder (`self.Cylinder`))
  ;[1 1 1] 변형
  (bind _asbp_third_person_character_1 (cast `/Game/Project/coin/BP_ThirdPersonCharacter1` OtherActor))
  (`/Game/Project/coin/BP_ThirdPersonCharacter1.Add Coins` _asbp_third_person_character_1)
  ;[1 1 1] 타이머 - Function
  (`SceneComponent.SetVisibility` _cylinder false false)
  (`PrimitiveComponent.SetCollisionEnabled` _cylinder "NoCollision")
  (`KismetSystemLibrary.K2_SetTimer` null "showcoin" 5.0)
  (`/Game/Project/coin/Bp_portal.Event Coin Over Lap` (`self.Portal`)))

(event `CustomEvent_1`
  ;[1 1 1] 코인 혼자서 도는 효과
  (`KismetSystemLibrary.K2_SetTimer` null "UpDateRotation" 0.01 true)
  (bind _outactors (`GameplayStatics.GetAllActorsOfClassWithTag` "/Game/Project/coin/Bp_portal.Bp_portal_C" "BTS"))
  (for _array_element _outactors
    (set `self.Portal` _array_element)
    ;[1 1 1] 코인 갯수 생성
    (bind _returnvalue (`|CreateWidget` "/Game/Project/coin/CoinCount.CoinCount_C"))
    (bind _output_get (set `self.text` _returnvalue))
    (`UserWidget.AddToViewport` _output_get 0)
    (`UserWidget.AddToViewport` _returnvalue 0)
    (for _ (range 10)
      _)))

(fn `showcoin`
  (bind _cylinder (`self.Cylinder`))
  (`SceneComponent.SetVisibility` _cylinder true false)
  (`PrimitiveComponent.SetCollisionEnabled` _cylinder "QueryAndPhysics"))

(fn `UpDateRotation`
  (`SceneComponent.K2_AddRelativeRotation` (`self.Cylinder`) (struct :`Yaw` 1.0) false false))

(fn `UserConstructionScript`)