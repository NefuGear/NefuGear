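; Spline mover actor that moves a static mesh back and forth along a spline between StartPlay and EndPlay calls.
; A timeline value scaled by the spline length gives a distance, which sets the mesh's world location without sweep on each update.
; When the timeline finishes, it flips IsRight and loops back to play or reverse, creating a ping-pong motion.
; BeginPlay is empty, and EndPlay stops the timeline.
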(event `/Game/Project/Bpi_MoveActer.StartPlay`
  (if (`self.Is Right`) :!label _label
    (bind (_direction _value) (`Timeline|타임라인` :!label _label_2)
      (:`Update`
        (`SceneComponent.K2_SetWorldLocation` (`self.StaticMesh`) (`SplineComponent.GetLocationAtDistanceAlongSpline` (`self.Spline`) (* _value (`SplineComponent.GetSplineLength` (`self.Spline`))) "World") false false))
      (:`Finished`
        (set `self.Is Right` (not (`self.Is Right`)))
        (goto _label)))
    (else
      (goto _label_2 :!via `Reverse`))))

(event `self.ReceiveBeginPlay`)

(event `/Game/Project/Bpi_MoveActer.EndPlay`
  (goto _label_2 :!via `Stop`))

(fn `UserConstructionScript`)