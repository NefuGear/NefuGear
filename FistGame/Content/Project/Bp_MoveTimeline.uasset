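; Actor Blueprint that slides a Cube component back and forth along its relative X axis using a Timeline, without relying on Tick.
; On BeginPlay it enables player input and plays the Timeline, whose value scaled by Distens sets the cube's location.
; On Finished it toggles IsRight to play or reverse, creating a ping-pong loop.
; T, K and L keys stop, play from start, or reverse from end.
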(event `self.ReceiveBeginPlay`
  (`self.EnableInput` (`GameplayStatics.GetPlayerController` 0))
  ;[1 1 1] Tick 없이도 자체적으로 타이밍을 조절한다.
  (bind (_direction _value) (`Timeline|타임라인` :`NewTime` 0.0 :!label _label)
    (:`Update`
      (`SceneComponent.K2_SetRelativeLocation` (`self.Cube`) (`KismetMathLibrary.MakeVector` (* _value (`self.Distens`))) false false))
    (:`Finished`
      (set `self.IsRight` (not (`self.IsRight`)))
      (if (`self.IsRight`)
        (goto _label)
        (else
          (goto _label :!via `Reverse`))))))

(event `Key|T`
  (params (Key :type "Key Structure"))
  (:`Pressed`
    (goto _label :!via `Stop`)))

(event `Key|K`
  (params (Key :type "Key Structure"))
  (:`Pressed`
    (goto _label :!via `PlayFromStart`)))

(event `Key|L`
  (params (Key :type "Key Structure"))
  (:`Pressed`
    (goto _label :!via `ReverseFromEnd`)))

(fn `UserConstructionScript`)