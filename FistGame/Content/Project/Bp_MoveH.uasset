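; Moving object Blueprint that loops its Cube component around a square path in the local XZ plane.
; While IsPlay is set, Tick offsets the Cube by Speed scaled by delta time along the current Setting direction.
; Passing a hardcoded bound switches Setting in the order Right, Up, Left, Down, without clamping the position.
; StartPlay and EndPlay events turn the motion on and off.
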(event `self.ReceiveTick`
  (params (DeltaSeconds :type "Float (single-precision)"))
  (bind _speed (`self.Speed`))
  (bind _cube (`self.Cube`))
  (bind _speed_2 (`self.Speed`))
  (bind _cube_2 (`self.Cube`))
  (bind (_relativelocation_x _relativelocation_y _relativelocation_z) (`KismetMathLibrary.BreakVector` (`SceneComponent.RelativeLocation` _cube)))
  (bind _relativelocation_x_2 (`KismetMathLibrary.BreakVector` (`SceneComponent.RelativeLocation` _cube_2)))
  (if (`self.IsPlay`)
    (switch `/Game/Project/EN_MoveType` (`self.Setting`)
      (:`NewEnumerator0`
        (`SceneComponent.K2_AddRelativeLocation` _cube_2 (`KismetMathLibrary.MakeVector` (* DeltaSeconds _speed_2)) false false)
        (if (>= _relativelocation_x_2 200.0)
          (set `self.Setting` "NewEnumerator2")))
      (:`NewEnumerator1`
        (`SceneComponent.K2_AddRelativeLocation` _cube_2 (`KismetMathLibrary.MakeVector` (* (* DeltaSeconds _speed_2) -1.0)) false false)
        (if (<= _relativelocation_x_2 0.0)
          (set `self.Setting` "NewEnumerator3")))
      (:`NewEnumerator2`
        (`SceneComponent.K2_AddRelativeLocation` _cube (`KismetMathLibrary.MakeVector` 0.0 0.0 (* DeltaSeconds _speed)) false false)
        (if (>= _relativelocation_z 200.0)
          (set `self.Setting` "NewEnumerator1")))
      (:`NewEnumerator3`
        (`SceneComponent.K2_AddRelativeLocation` _cube (`KismetMathLibrary.MakeVector` 0.0 0.0 (* (* DeltaSeconds _speed) -1.0)) false false)
        (if (<= _relativelocation_z 0.0)
          (set `self.Setting` "NewEnumerator0"))))))

(event `/Game/Project/Bpi_MoveActer.StartPlay`
  (set `self.IsPlay` true))

(event `/Game/Project/Bpi_MoveActer.EndPlay`
  (set `self.IsPlay` false))

(fn `UserConstructionScript`)