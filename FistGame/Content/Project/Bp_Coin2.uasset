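; Coin pickup actor that spins its cylinder mesh a fixed step every tick.
; When BP_ThirdPersonCharacter1 overlaps the cylinder, it adds to that character's coins, destroys itself and notifies a Portal through EventCoinOverLap.
; On BeginPlay each coin creates its own CoinCount widget and adds it to the viewport, then runs an empty loop.
; A spawn-sound node is present but never runs.
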(event `self.Cylinder.OnComponentBeginOverlap`
  (params (OverlappedComponent :type "PrimitiveComponent Object Reference") (OtherActor :type "Actor Object Reference") (OtherComp :type "PrimitiveComponent Object Reference") (OtherBodyIndex :type Integer) (bFromSweep :type Boolean) (SweepResult :type "HitResult Structure (by ref)"))
  ;[1 1 1] 변형
  (bind _asbp_third_person_character_1 (cast `/Game/Project/coin/BP_ThirdPersonCharacter1` OtherActor))
  (`/Game/Project/coin/BP_ThirdPersonCharacter1.Add Coins` _asbp_third_person_character_1)
  (`self.K2_DestroyActor`)
  (`/Game/Project/coin/Bp_portal.EventCoinOverLap` (`self.Portal`)))

(event `self.ReceiveTick`
  (params (DeltaSeconds :type "Float (single-precision)"))
  (`SceneComponent.K2_AddRelativeRotation` (`self.Cylinder`) (struct :`Yaw` 1.5) false false))

(event `self.ReceiveBeginPlay`
  ;[1 1 1] 변형
  (bind _returnvalue (`|CreateWidget` "/Game/Project/coin/CoinCount.CoinCount_C"))
  (bind _output_get (set `self.text` _returnvalue))
  (`UserWidget.AddToViewport` _output_get 0)
  (`UserWidget.AddToViewport` _returnvalue 0)
  (for _ (range 10)
    _))

(fn `UserConstructionScript`)