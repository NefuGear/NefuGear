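; Switch panel that starts and stops linked moving actors while something overlaps its Cube.
; Begin overlap loops through the Acters array, casts each entry to Bp_MoveH or Bp_MoveSpline, and sends StartPlayMessage through the Bpi_MoveActer interface.
; End overlap repeats the same loop to send EndPlayMessage.
; Neither event filters the overlapping actor or counts how many overlaps remain.
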(event `self.Cube.OnComponentBeginOverlap`
  (params (OverlappedComponent :type "PrimitiveComponent Object Reference") (OtherActor :type "Actor Object Reference") (OtherComp :type "PrimitiveComponent Object Reference") (OtherBodyIndex :type Integer) (bFromSweep :type Boolean) (SweepResult :type "HitResult Structure (by ref)"))
  (for _array_element (`self.Acters`)
    (bind _asbp_move_h (cast `/Game/Project/Bp_MoveH` _array_element)
      (:`then`
        (if (`KismetSystemLibrary.DoesImplementInterface` _asbp_move_h "/Game/Project/Bpi_MoveActer.Bpi_MoveActer_C")
          (message `/Game/Project/Bpi_MoveActer.StartPlay` _asbp_move_h)))
      (:`CastFailed`
        (bind _asbp_move_spline (cast `/Game/Project/Bp_MoveSpline` _array_element))
        (if (`KismetSystemLibrary.DoesImplementInterface` _asbp_move_spline "/Game/Project/Bpi_MoveActer.Bpi_MoveActer_C")
          (message `/Game/Project/Bpi_MoveActer.StartPlay` _asbp_move_spline))))))

(event `self.Cube.OnComponentEndOverlap`
  (params (OverlappedComponent :type "PrimitiveComponent Object Reference") (OtherActor :type "Actor Object Reference") (OtherComp :type "PrimitiveComponent Object Reference") (OtherBodyIndex :type Integer))
  (for _array_element (`self.Acters`)
    (bind _asbp_move_h (cast `/Game/Project/Bp_MoveH` _array_element)
      (:`then`
        (if (`KismetSystemLibrary.DoesImplementInterface` _asbp_move_h "/Game/Project/Bpi_MoveActer.Bpi_MoveActer_C")
          (message `/Game/Project/Bpi_MoveActer.EndPlay` _asbp_move_h)))
      (:`CastFailed`
        (bind _asbp_move_spline (cast `/Game/Project/Bp_MoveSpline` _array_element))
        (if (`KismetSystemLibrary.DoesImplementInterface` _asbp_move_spline "/Game/Project/Bpi_MoveActer.Bpi_MoveActer_C")
          (message `/Game/Project/Bpi_MoveActer.EndPlay` _asbp_move_spline))))))

(fn `UserConstructionScript`)