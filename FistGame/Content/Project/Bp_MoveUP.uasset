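; Blueprint that slides a Sphere component back and forth along its relative X axis between two fixed limits.
; Tick moves the sphere by Speed scaled by delta time while IsPlay is true, flipping the IsRight flag at each limit to reverse direction.
; StartPlay and EndPlay events switch the motion on and off by setting IsPlay.
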(event `self.ReceiveTick`
  (params (DeltaSeconds :type "Float (single-precision)"))
  (bind _speed (`self.Speed`))
  (bind _sphere (`self.Sphere`))
  (bind _relativelocation_x (`KismetMathLibrary.BreakVector` (`SceneComponent.RelativeLocation` _sphere)))
  (if (`self.IsPlay`)
    (if (`self.IsRight`)
      (`SceneComponent.K2_AddRelativeLocation` _sphere (`KismetMathLibrary.MakeVector` (* DeltaSeconds _speed)) false false)
      (if (>= _relativelocation_x 200.0)
        (set `self.IsRight` false))
      (else
        (`SceneComponent.K2_AddRelativeLocation` _sphere (`KismetMathLibrary.MakeVector` (* (* DeltaSeconds _speed) -1.0)) false false)
        (if (<= _relativelocation_x 0.0)
          (set `self.IsRight` true))))))

(event `/Game/Project/Bpi_MoveActer.StartPlay`
  (set `self.IsPlay` true))

(event `/Game/Project/Bpi_MoveActer.EndPlay`
  (set `self.IsPlay` false))

(fn `UserConstructionScript`)