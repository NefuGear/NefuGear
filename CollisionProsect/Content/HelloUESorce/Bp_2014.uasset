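; Practice-style Blueprint that moves its Sphere component around a square loop in the local X-Z plane while IsPlay is true.
; Tick switches on the Seter direction state (Right, Up, Left, Down) and calls one movement function per side, scaled by Speed2 and delta time.
; Each function offsets the sphere and advances the state once its relative location passes the 0 or 200 unit boundary.
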(event `self.ReceiveBeginPlay`)

(event `self.ReceiveTick`
  (params (DeltaSeconds :type "Float (single-precision)"))
  (bind _sphere (`self.Sphere`))
  (bind _sphere_2 (`self.Sphere`))
  (bind _speed2 (`self.Speed2`))
  (bind _speed2_2 (`self.Speed2`))
  (bind (_relativelocation_x _relativelocation_y _relativelocation_z) (`KismetMathLibrary.BreakVector` (`SceneComponent.RelativeLocation` _sphere)))
  (bind _relativelocation_x_2 (`KismetMathLibrary.BreakVector` (`SceneComponent.RelativeLocation` _sphere_2)))
  (if (`self.Is Play`)
    (switch `/Game/HelloUESorce/En_MoveType` (`self.Seter`)
      (:`NewEnumerator4`
        ;[1 1 1] 이동 스메시
        ;;[0 0.05611 1 1 20] 오른쪽 전진
        (`self.Move Right` _speed2 DeltaSeconds _sphere_2 (>= _relativelocation_x_2 200.0)))
      (:`NewEnumerator5`
        ;[1 1 1] 이동스메시
        ;;[0 0.05611 1 1 20] 위로 전진
        (`self.NewFunction` DeltaSeconds _speed2_2 _sphere (>= _relativelocation_z 200.0)))
      (:`NewEnumerator6`
        ;;[1 0 0.009549 1 20] 왼쪽 전진
        (`self.Move Left` DeltaSeconds _speed2 _sphere_2 (<= _relativelocation_x_2 0.0)))
      (:`NewEnumerator7`
        ;;[1 0 0.009549 1 20] 아래로 전진
        (`self.NewFunction_0` DeltaSeconds _speed2_2 (<= _relativelocation_z 0.0) _sphere)))))

(fn `Move Left`
  (params (A :type "Float (double-precision)") (B :type "Float (double-precision)") (InputPin :type "StaticMeshComponent Object Reference") (InputPin2 :type Boolean))
  (`SceneComponent.K2_AddRelativeLocation` InputPin (`KismetMathLibrary.MakeVector` (* (* A B) -1.0)) false false)
  (if InputPin2
    (set `self.Seter` "NewEnumerator7")))

(fn `Move Right`
  (params (A :type "Float (double-precision)") (B :type "Float (double-precision)") (self2 :type "SceneComponent Object Reference") (Condition :type Boolean))
  (`SceneComponent.K2_AddRelativeLocation` self2 (`KismetMathLibrary.MakeVector` (* A B)) false false)
  (if Condition
    (set `self.Seter` "NewEnumerator5")))

(fn `NewFunction`
  (params (A :type "Float (double-precision)") (B :type "Float (double-precision)") (self2 :type "SceneComponent Object Reference") (Condition :type Boolean))
  (`SceneComponent.K2_AddRelativeLocation` self2 (`KismetMathLibrary.MakeVector` 0.0 0.0 (* A B)) false false)
  (if Condition
    (set `self.Seter` "NewEnumerator6")))

(fn `NewFunction_0`
  (params (A :type "Float (double-precision)") (B :type "Float (double-precision)") (Condition :type Boolean) (InputPin :type "StaticMeshComponent Object Reference"))
  (`SceneComponent.K2_AddRelativeLocation` InputPin (`KismetMathLibrary.MakeVector` 0.0 0.0 (* (* A B) -1.0)) false false)
  (if Condition
    (set `self.Seter` "NewEnumerator4")))

(fn `UserConstructionScript`)