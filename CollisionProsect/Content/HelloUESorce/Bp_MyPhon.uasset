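; Player-controlled pawn that flies freely along its own axes and turns the view with look input.
; Forward, right and up input axes offset the actor along its matching direction vectors by a fixed step per axis event, without sweep or delta-time scaling, so movement ignores collision and depends on frame rate.
; Two further axes feed controller yaw and pitch.
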(event `InputAxis|MoveForWoard`
  (params (AxisValue :type "Float (single-precision)"))
  ;[1 1 1] 앞 뒤 셋팅
  (`self.K2_AddActorWorldOffset` (* (`self.GetActorForwardVector`) (* AxisValue 10.0))))

(event `InputAxis|MoveRight`
  (params (AxisValue :type "Float (single-precision)"))
  ;[1 1 1] 왼 오 셋팅
  (`self.K2_AddActorWorldOffset` (* (`self.GetActorRightVector`) (* AxisValue 10.0))))

(event `InputAxis|MoveM_right`
  (params (AxisValue :type "Float (single-precision)"))
  ;[1 1 1] 마우스 시점변화
  (`self.AddControllerYawInput` AxisValue))

(event `InputAxis|MoveUp`
  (params (AxisValue :type "Float (single-precision)"))
  ;[1 1 1] 위 아래 셋팅
  (`self.K2_AddActorWorldOffset` (* (`self.GetActorUpVector`) (* AxisValue 10.0))))

(event `InputAxis|MoveM_up`
  (params (AxisValue :type "Float (single-precision)"))
  ;[1 1 1] 마우스 시점변화
  (`self.AddControllerPitchInput` AxisValue))

(fn `UserConstructionScript`)